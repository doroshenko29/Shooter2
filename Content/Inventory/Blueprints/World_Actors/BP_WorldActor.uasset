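; World actor that represents an inventory item in the level, with a mesh and a floating name widget.
; On BeginPlay it reads the ItemSignature from the Item class defaults to set the mesh and pass name, stackability and Amount to WB_WorldItem.
; Every Tick it rotates the widget component to face the player character's camera, billboard style.
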(event `self.ReceiveBeginPlay`
  (`self.Initialize 3D Mesh`)
  (`self.Initialize Item Name`))

(event `self.ReceiveTick`
  (params (DeltaSeconds :type "Float (single-precision)"))
  (`self.Update Widget Rotation`))

(fn `Initialize 3D Mesh`
  (`StaticMeshComponent.SetStaticMesh` (`self.ItemMesh`) (`.3DMesh_18_5BA81D9740DA4C029EF08B8FEF0ED137` (break `/Game/Inventory/Structures/S_ItemSigniture` (defaults `/Game/Inventory/Blueprints/World_Actors/BP_WorldActor` (`self.Item`))))))

(fn `Initialize Item Name`
  (bind _item_signature (defaults `/Game/Inventory/Blueprints/World_Actors/BP_WorldActor` (`self.Item`)))
  (bind _aswb_world_item (cast `/Game/Inventory/UI/WB_WorldItem` (`WidgetComponent.GetUserWidgetObject` (`self.Item WB`))))
  (`/Game/Inventory/UI/WB_WorldItem.Set Item Name` _aswb_world_item (break `/Game/Inventory/Structures/S_ItemSigniture` _item_signature) (`.Stackable_12_F7FCE8164DB3FE3580C627B872EB4D51` (break `/Game/Inventory/Structures/S_ItemSigniture` _item_signature)) (`self.Amount`)))

(fn `Update Widget Rotation`
  (`SceneComponent.K2_SetWorldRotation` (`self.Item WB`) (`KismetMathLibrary.FindLookAtRotation` (`SceneComponent.K2_GetComponentLocation` (`self.Item WB`)) (`SceneComponent.K2_GetComponentLocation` (`/Game/Blueprints/Player/BP_PlayerCharacter.Camera` (cast `/Game/Blueprints/Player/BP_PlayerCharacter` (`GameplayStatics.GetPlayerCharacter` 0) :!pure true)))) false false))

(fn `UserConstructionScript`)