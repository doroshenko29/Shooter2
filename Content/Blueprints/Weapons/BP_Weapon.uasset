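; BP_Weapon is a weapon Blueprint that handles ammo, fire-rate limiting and firing feedback.
; UseWeapon checks ammo and the rate lock, then spends a round, plays the shot sound, widens the player crosshair and returns true.
; A timer calling StopRateDelay releases the lock after UseRate.
; Any blocked shot, including during the rate delay, prints a reload message, plays the out-of-ammo sound and returns false.
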(fn `AbleToUseWeapon`
  (returns (Out :type Boolean))
  (return (and (> (`self.CurrentAmmo`) 0) (not (`self.UseFreezeByRate`)))))

(fn `StopRateDelay`
  (set `self.UseFreezeByRate` false))

(fn `UserConstructionScript`)

(fn `UseWeapon`
  (returns (Used :type Boolean))
  (if (`self.AbleToUseWeapon`)
    (`/Engine/EditorBlueprintResources/StandardMacros.DecrementInt` (`self.CurrentAmmo`)
      (:`  `
        ;[1 1 1] Если игра в конечном счёте будет иметь онлайн, то это может и не подойти. Звук услышим только мы.. Тут надо будет тупо добавить радиус вектор, на котором мы хотим слышать звук
        ;;[1 0 0.07149] проигрываем звук, только в случае, если произошёл выстрел! Если делать это в BP_PlayerCharacter - звук будет проигрывать всегда, когда мы нажимаем на ЛКМ, т.к. никаких условий мы там не ставим
        (`GameplayStatics.PlaySoundAtLocation` "/Game/Assets/Characters/FirstPerson/Audio/FirstPersonTemplateWeaponFire02.FirstPersonTemplateWeaponFire02" (`self.K2_GetActorLocation`) (struct) 1.0 1.0 0.0 null null null) ; Play firing sound
        ;[1 0.06102 0] меняем размер, аналогично предыдущему комменту
        (`/Game/Blueprints/Player/BP_PlayerCharacter.Change Size Of Crosshair` (cast `/Game/Blueprints/Player/BP_PlayerCharacter` (`GameplayStatics.GetPlayerCharacter` 0) :!pure true) 20.0 60.0)
        (`KismetSystemLibrary.K2_SetTimer` null "StopRateDelay" (`self.UseRate`))
        (set `self.UseFreezeByRate` true)
        (return true)))
    (else
      ;[1 1 1] думаю , тут можно будет реализовать необходимость перезарядки(звук того что нет патронов в патроннике ну и можно писать - перезарядись )
      (`KismetSystemLibrary.PrintString` "перезарядка..." true true (struct :`G` 0.66 :`B` 1.0 :`A` 1.0) 0.5)
      (`GameplayStatics.PlaySoundAtLocation` "/Game/Assets/Audio/out_Of_Ammo.out_Of_Ammo" (`self.K2_GetActorLocation`) (struct) 1.0 1.0 0.0 null null null)
      (return false))))